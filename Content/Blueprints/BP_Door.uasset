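; An interactable door Blueprint that swings its static mesh open and closed on yaw.
; Interact calls DoorActivate and returns false; after a short delay, the IsDoorClosed flag selects one of two timelines.
; Timeline_0 plays forward to open and Timeline_1 plays in reverse to close, each lerping between the DoorClosed and DoorOpen angles.
; The flag flips only when a timeline finishes.
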(event `DoorActivate`
  (`KismetSystemLibrary.Delay` 0.2)
  (if (`self.IsDoorClosed?`)
    (bind (_direction _open_close) (`Timeline|Timeline_0` :!via `PlayFromStart`)
      (:`Update`
        (`SceneComponent.K2_SetRelativeRotation` (`self.StaticMesh`) (`KismetMathLibrary.MakeRotator` 0.0 0.0 (`KismetMathLibrary.Lerp` (`self.DoorClosed`) (`self.DoorOpen`) _open_close)) false false))
      (:`Finished`
        (set `self.IsDoorClosed?` false)))
    (else
      (bind (_direction_2 _open_close_2) (`Timeline|Timeline_1` :!via `ReverseFromEnd`)
        (:`Update`
          (`SceneComponent.K2_SetRelativeRotation` (`self.StaticMesh`) (`KismetMathLibrary.MakeRotator` 0.0 0.0 (`KismetMathLibrary.Lerp` (`self.DoorClosed`) (`self.DoorOpen`) _open_close_2)) false false))
        (:`Finished`
          (set `self.IsDoorClosed?` true))))))

(fn `Interact`
  (returns (SuccessfulInteract :type Boolean))
  (`self.DoorActivate`)
  (return false))

(fn `UserConstructionScript`)