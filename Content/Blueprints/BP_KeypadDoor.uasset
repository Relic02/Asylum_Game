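; Locked door actor that opens by keypad code or offers a crowbar bash, and ends the game with a win screen.
; CheckCode accepts or declines the code, setting the lock and activating timeline-driven rotation; first opening shows YouWin and pauses.
; A box trigger prompts crowbar holders when locked; Use then starts bash widgets, and Bash animates door and crowbar.
; A second trigger plays a one-time sound for EvilPlayer-tagged actors.
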(event `self.ReceiveBeginPlay`
  (bind _askeypad_w (cast `/Game/Widgets/Keypad_W` (`WidgetComponent.GetUserWidgetObject` (`self.KeypadWidget`))))
  (bind _output_get (set `self.As Keypad W` _askeypad_w))
  (add `/Game/Widgets/Keypad_W.CodeEntered` _output_get (`|CreateDelegate` :!event `CheckCode`)))

(event `/Game/Interfaces/InteractInterface.Use`
  (params (Actor :type "/Game/FirstPerson/Blueprints/BP_FirstPersonCharacter Object Reference"))
  (bind _returnvalue (`GameplayStatics.GetPlayerController` 0))
  (if (`self.BashWidgetUp?`)
    (bind _returnvalue_2 (`|CreateWidget` "/Game/Widgets/DoorBash/DoorBash1.DoorBash1_C"))
    (`UserWidget.AddToViewport` _returnvalue_2 0)
    (`SceneComponent.SetVisibility` (`self.Crowbar`) true false)
    (else
      (`KismetSystemLibrary.Delay` 0.2 :!label _label)
      (if (`self.IsLocked`)
        _
        (elif (`self.IsDoorClosed?`)
          (bind (_direction _open_close) (`Timeline|Timeline_0` :!via `PlayFromStart`)
            (:`Update`
              (`SceneComponent.K2_SetRelativeRotation` (`self.Door`) (`KismetMathLibrary.MakeRotator` 0.0 0.0 (`KismetMathLibrary.Lerp` (`self.LeftPanelClosed`) (`self.LeftPanelOpen`) _open_close)) false false))
            (:`Finished`
              (set `self.IsDoorClosed?` false)
              (bind _asbp_first_person_character (cast `/Game/FirstPerson/Blueprints/BP_FirstPersonCharacter` (`self.As BP First Person Character`)))
              (bind _output_get (set `self.As BP First Person Character` _asbp_first_person_character))
              (`/Game/FirstPerson/Blueprints/BP_FirstPersonCharacter.StopCamShake` _output_get)
              (`/Engine/EditorBlueprintResources/StandardMacros.DoOnce` false
                (:`Completed`
                  (bind _returnvalue_3 (`|CreateWidget` "/Game/Widgets/YouWin.YouWin_C"))
                  (`UserWidget.AddToViewport` _returnvalue_3 0)
                  (set `PlayerController.bShowMouseCursor` true _returnvalue)
                  (`WidgetBlueprintLibrary.SetInputMode_GameAndUIEx` _returnvalue _returnvalue_3)
                  (`GameplayStatics.SetGamePaused` true)
                  (`GameplayStatics.PlaySound2D` "/Game/AIDoctor/SFX/Sweet_Lamb.Sweet_Lamb" 1.0 1.0 0.0 null null)))))
          (else
            (bind (_direction_2 _open_close_2) (`Timeline|Timeline_1` :!via `ReverseFromEnd`)
              (:`Update`
                (`SceneComponent.K2_SetRelativeRotation` (`self.Door`) (`KismetMathLibrary.MakeRotator` 0.0 0.0 (`KismetMathLibrary.Lerp` (`self.LeftPanelClosed`) (`self.LeftPanelOpen`) _open_close_2)) false false))
              (:`Finished`
                (set `self.IsDoorClosed?` true)))))))))

(event `DoorActivate`
  (goto _label))

(event `LockDoor`
  (set `self.IsLocked` true))

(event `UnlockDoor`
  (set `self.IsLocked` false))

(event `Bash`
  (if (`self.Bashable`)
    (`|ExecutionSequence`
      (:`then_0`
        (bind (_direction _newtrack_0) (`Timeline|DoorBash` :!via `PlayFromStart`)
          (:`Update`
            (`SceneComponent.K2_SetRelativeRotation` (`self.Door`) (`KismetMathLibrary.MakeRotator` 0.0 0.0 (`KismetMathLibrary.Lerp` (`self.LeftPanelClosed`) (`self.BashValue`) _newtrack_0)) false false))
          (:`Finished`
            (set `self.Bashable` true))))
      (:`then_1`
        (`Timeline|Crowbaryank` :!via `PlayFromStart`
          (:`Update`
            (`SceneComponent.K2_SetRelativeRotation` (`self.Crowbar`) (`KismetMathLibrary.MakeRotator` (`KismetMathLibrary.Lerp` (`self.CrowbarStartPos`) (`self.CrowbarBashPos`) _newtrack_0) -90.0) false false)))))))

(event `self.Box.OnComponentBeginOverlap`
  (params (OverlappedComponent :type "PrimitiveComponent Object Reference") (OtherActor :type "Actor Object Reference") (OtherComp :type "PrimitiveComponent Object Reference") (OtherBodyIndex :type Integer) (bFromSweep :type Boolean) (SweepResult :type "HitResult Structure (by ref)"))
  (if (`self.IsLocked`)
    (bind _asbp_first_person_character (cast `/Game/FirstPerson/Blueprints/BP_FirstPersonCharacter` OtherActor))
    (bind _output_get (set `self.As BP First Person Character` _asbp_first_person_character))
    (if (`/Game/FirstPerson/Blueprints/BP_FirstPersonCharacter.HasCrowbar?` _output_get)
      (bind _returnvalue (`|CreateWidget` "/Game/Widgets/Notifications/CrowbarUse_W.CrowbarUse_W_C"))
      (`UserWidget.AddToViewport` _returnvalue 0)
      (set `self.BashWidgetUp?` true))))

(event `self.Box.OnComponentEndOverlap`
  (params (OverlappedComponent :type "PrimitiveComponent Object Reference") (OtherActor :type "Actor Object Reference") (OtherComp :type "PrimitiveComponent Object Reference") (OtherBodyIndex :type Integer))
  (if (`self.BashWidgetUp?`)
    (`Widget.RemoveFromParent` (stale `self.Box.OnComponentBeginOverlap` _returnvalue))
    (set `self.BashWidgetUp?` false)
    (`|ExecutionSequence`
      (:`then_0`
        (bind _foundwidgets (`WidgetBlueprintLibrary.GetAllWidgetsOfClass` "/Game/Widgets/DoorBash/DoorBash1.DoorBash1_C"))
        (`/Engine/EditorBlueprintResources/StandardMacros.IsValid` (`|GetArrayItem` _foundwidgets)
          (:`Is Valid`
            _)))
      (:`then_1`
        (bind _foundwidgets_2 (`WidgetBlueprintLibrary.GetAllWidgetsOfClass` "/Game/Widgets/DoorBash/DoorBash2.DoorBash2_C"))
        (bind _output (`|GetArrayItem` _foundwidgets_2))
        (`/Engine/EditorBlueprintResources/StandardMacros.IsValid` _output
          (:`Is Valid`
            _)))
      (:`then_2`
        (bind _foundwidgets_3 (`WidgetBlueprintLibrary.GetAllWidgetsOfClass` "/Game/Widgets/DoorBash/DoorBreak.DoorBreak_C"))
        (`/Engine/EditorBlueprintResources/StandardMacros.IsValid` (`|GetArrayItem` _foundwidgets_3)
          (:`Is Valid`
            _))))
    (`Widget.RemoveFromParent` _output)
    (`Widget.RemoveFromParent` (`|GetArrayItem` _foundwidgets_3))
    (`Widget.RemoveFromParent` (`|GetArrayItem` _foundwidgets))))

(event `self.AudiopTrig.OnComponentBeginOverlap`
  (params (OverlappedComponent :type "PrimitiveComponent Object Reference") (OtherActor :type "Actor Object Reference") (OtherComp :type "PrimitiveComponent Object Reference") (OtherBodyIndex :type Integer) (bFromSweep :type Boolean) (SweepResult :type "HitResult Structure (by ref)"))
  (if (`self.ActorHasTag` OtherActor "EvilPlayer")
    (if (not (`self.played sound`))
      (`GameplayStatics.PlaySound2D` "/Game/SFX/Player/Old_door.Old_door" 1.5 1.0 0.0 null null)
      (set `self.played sound` true))))

(fn `CheckCode`
  (params (Code :type String) (KeyPad :type "/Game/Widgets/Keypad_W Object Reference"))
  (if (`KismetStringLibrary.EqualEqual_StrStr` Code (`self.CorrectCode`))
    (`self.CodeAccept`)
    (`self.UnlockDoor`)
    (`self.DoorActivate`)
    (set `/Game/Widgets/Keypad_W.CurrentCode` "" KeyPad)
    (else
      (`self.CodeDecline`)
      (`self.LockDoor`)
      (set `/Game/Widgets/Keypad_W.CurrentCode` "" KeyPad))))

(fn `UserConstructionScript`)