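; BP_MasterKey is a key pickup whose KeyColor selects a type: Cage, Door 1 or Door 2.
; The construction script adds KeyColor to the actor's tags and sets the mesh material by type, with only Cage assigning a named material.
; Use adds the key to the passed actor's Keys array without duplicates and hides it rather than destroying it.
; It then shows a KeyAcquired_W notification for player 0 and removes it after a short delay.
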(event `/Game/Interfaces/InteractInterface.Use`
  (params (Actor :type "/Game/FirstPerson/Blueprints/BP_FirstPersonCharacter Object Reference"))
  (`KismetArrayLibrary.Array_AddUnique` (`/Game/FirstPerson/Blueprints/BP_FirstPersonCharacter.Keys` Actor) self)
  (`self.SetActorHiddenInGame` true)
  (bind _returnvalue (`|CreateWidget` "/Game/Widgets/Notifications/KeyAcquired_W.KeyAcquired_W_C" (`GameplayStatics.GetPlayerController` 0)))
  (`UserWidget.AddToViewport` _returnvalue 0)
  (`KismetSystemLibrary.Delay` 2.0)
  (`Widget.RemoveFromParent` _returnvalue))

(fn `UserConstructionScript`
  (bind _keycolor (`self.KeyColor`))
  (bind _staticmesh (`self.StaticMesh`))
  (`KismetArrayLibrary.Array_AddUnique` (`self.Tags`) _keycolor)
  (switch `name` _keycolor
    (:`Cage`
      (`PrimitiveComponent.SetMaterial` _staticmesh 0 "/Engine/VREditor/LaserPointer/M_LaserPointer-Core.M_LaserPointer-Core"))
    (:`Door1`
      (`PrimitiveComponent.SetMaterial` _staticmesh 0 null))
    (:`Door2`
      (`PrimitiveComponent.SetMaterial` _staticmesh 0 null))))