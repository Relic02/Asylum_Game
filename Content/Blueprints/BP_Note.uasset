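; BP_Note is an interactable note that shows a Note_W widget on screen when used.
; Overlapping its Sphere caches a player controller, looked up with the overlap's body index as the player index.
; Use calls ReadNote, which creates the widget with that controller as owner and adds it to the viewport.
; The UI-only input mode and mouse cursor logic is unconnected and never runs.
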(event `ReadNote`
  (bind _returnvalue (`|CreateWidget` "/Game/Widgets/Note_W.Note_W_C" (`self.Controller`)))
  (`UserWidget.AddToViewport` _returnvalue 0))

(event `self.Sphere.OnComponentBeginOverlap`
  (params (OverlappedComponent :type "PrimitiveComponent Object Reference") (OtherActor :type "Actor Object Reference") (OtherComp :type "PrimitiveComponent Object Reference") (OtherBodyIndex :type Integer) (bFromSweep :type Boolean) (SweepResult :type "HitResult Structure (by ref)"))
  (set `self.Controller` (`GameplayStatics.GetPlayerController` OtherBodyIndex)))

(fn `Use`
  (params (Actor :type "/Game/FirstPerson/Blueprints/BP_FirstPersonCharacter Object Reference"))
  (`self.ReadNote`)
  (return))

(fn `UserConstructionScript`)