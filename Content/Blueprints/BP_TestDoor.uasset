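; Swinging door that the Use event opens or closes, with an optional key lock.
; When locked, Use clears the user's Keys array and unlocks, or briefly shows a need-key widget if none is held.
; Timelines lerp the door's yaw between closed and open angles, with InMotion blocking re-triggers.
; Actors tagged "Doc" open it on AIOverlap unless AiLock is set, which player-style Use clears.
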(event `/Game/Interfaces/InteractInterface.Use`
  (params (Actor :type "/Game/FirstPerson/Blueprints/BP_FirstPersonCharacter Object Reference"))
  (bind _keys (`/Game/FirstPerson/Blueprints/BP_FirstPersonCharacter.Keys` Actor))
  (if (`self.Needsakey`)
    (`/Engine/EditorBlueprintResources/StandardMacros.IsValid` (`|GetArrayItem` _keys)
      (:`Is Valid`
        (`KismetArrayLibrary.Array_Clear` _keys)
        (`|ExecutionSequence`
          (:`then_0`
            (bind _returnvalue (`|CreateWidget` "/Game/Widgets/KeyUSed_W.KeyUSed_W_C"))
            (`UserWidget.AddToViewport` _returnvalue 0)
            (`KismetSystemLibrary.Delay` 2.0)
            (`Widget.RemoveFromParent` _returnvalue))
          (:`then_1`
            (set `self.Needsakey` false)
            (if (not (`self.InMotion?`)) :!label _label
              (set `self.AiLock` false)
              (if (`self.IsDoorClosed`)
                (bind (_direction _open_close) (`Timeline|DoorOpen` :!via `PlayFromStart`)
                  (:`Update`
                    (set `self.InMotion?` true)
                    (`SceneComponent.K2_SetRelativeRotation` (`self.Door`) (`KismetMathLibrary.MakeRotator` 0.0 0.0 (`KismetMathLibrary.Lerp` (`self.ClosedAngle`) (`self.OpenAngle`) _open_close)) false false))
                  (:`Finished`
                    (set `self.IsDoorClosed` false)
                    (set `self.InMotion?` false)))
                (else
                  (bind (_direction_2 _open_close_2) (`Timeline|Timeline_0` :!via `ReverseFromEnd`)
                    (:`Update`
                      (set `self.InMotion?` true)
                      (`SceneComponent.K2_SetRelativeRotation` (`self.Door`) (`KismetMathLibrary.MakeRotator` 0.0 0.0 (`KismetMathLibrary.Lerp` (`self.ClosedAngle`) (`self.OpenAngle`) _open_close_2)) false false))
                    (:`Finished`
                      (set `self.IsDoorClosed` true)
                      (set `self.InMotion?` false)))))))))
      (:`Is Not Valid`
        (bind _returnvalue_2 (`|CreateWidget` "/Game/Widgets/NeedKey_W.NeedKey_W_C"))
        (`UserWidget.AddToViewport` _returnvalue_2 0)
        (`KismetSystemLibrary.Delay` 2.0)
        (`Widget.RemoveFromParent` _returnvalue_2)))
    (else
      (goto _label))))

(event `self.AIOverlap.OnComponentBeginOverlap`
  (params (OverlappedComponent :type "PrimitiveComponent Object Reference") (OtherActor :type "Actor Object Reference") (OtherComp :type "PrimitiveComponent Object Reference") (OtherBodyIndex :type Integer) (bFromSweep :type Boolean) (SweepResult :type "HitResult Structure (by ref)"))
  (if (`self.ActorHasTag` OtherActor "Doc")
    (if (`self.AiLock`)
      _
      (elif (`self.InMotion?`)
        _
        (elif (`self.IsDoorClosed`)
          (bind (_direction _open_close) (`Timeline|Timeline_1` :!via `PlayFromStart`)
            (:`Update`
              (set `self.InMotion?` true)
              (`SceneComponent.K2_SetRelativeRotation` (`self.Door`) (`KismetMathLibrary.MakeRotator` 0.0 0.0 (`KismetMathLibrary.Lerp` (`self.ClosedAngle`) (`self.OpenAngle`) _open_close)) false false))
            (:`Finished`
              (set `self.IsDoorClosed` false)
              (set `self.InMotion?` false))))))))

(fn `UserConstructionScript`)