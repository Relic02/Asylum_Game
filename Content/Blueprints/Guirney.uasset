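; Gurney actor whose mattress the player can cut open to reveal a key.
; Overlapping the Box caches the first-person character and, if it has a cutting tool and the mattress is uncut, briefly shows the Matresscut widget.
; Use checks that cached character for the tool, then makes the key and open-mattress mesh visible and sets BeenCut, which suppresses later prompts.
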(event `/Game/Interfaces/InteractInterface.Use`
  (params (Actor :type "/Game/FirstPerson/Blueprints/BP_FirstPersonCharacter Object Reference"))
  (if (`/Game/FirstPerson/Blueprints/BP_FirstPersonCharacter.HasCuttingTool?` (`self.As BP First Person Character`))
    (`SceneComponent.SetVisibility` (`self.Key`) true false)
    (`SceneComponent.SetVisibility` (`self.SM_MatressOpen`) true false)
    (set `self.BeenCut` true)))

(event `self.Box.OnComponentBeginOverlap`
  (params (OverlappedComponent :type "PrimitiveComponent Object Reference") (OtherActor :type "Actor Object Reference") (OtherComp :type "PrimitiveComponent Object Reference") (OtherBodyIndex :type Integer) (bFromSweep :type Boolean) (SweepResult :type "HitResult Structure (by ref)"))
  (bind _asbp_first_person_character (cast `/Game/FirstPerson/Blueprints/BP_FirstPersonCharacter` OtherActor))
  (set `self.As BP First Person Character` _asbp_first_person_character)
  (if (`self.BeenCut`)
    _
    (elif (`/Game/FirstPerson/Blueprints/BP_FirstPersonCharacter.HasCuttingTool?` (`self.As BP First Person Character`))
      (bind _returnvalue (`|CreateWidget` "/Game/Widgets/Notifications/Matresscut.Matresscut_C" (`GameplayStatics.GetPlayerController` 0)))
      (`UserWidget.AddToViewport` _returnvalue 0)
      (`KismetSystemLibrary.Delay` 1.0)
      (`Widget.RemoveFromParent` _returnvalue))))

(fn `UserConstructionScript`)