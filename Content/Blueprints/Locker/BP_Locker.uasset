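; BP_Locker is a locker the player can hide in, toggled through its Use event.
; ToggleHide flips the hiding state on locker and player, hides the player, disables their collision and blends the view to the locker, reversing this on exit.
; Each use also plays the OpenDoor timeline from the start, lerping door yaw between closed and open angles.
; Box overlap events are empty, with leftover input and camera nodes disconnected.
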(event `/Game/Interfaces/InteractInterface.Use`
  (params (Actor :type "/Game/FirstPerson/Blueprints/BP_FirstPersonCharacter Object Reference"))
  ;[1 1 1] In/OutLocker
  (set `self.PlayerRef` Actor)
  (`|ExecutionSequence`
    (:`then_0`
      (`self.ToggleHide`)
      (`KismetSystemLibrary.Delay` 0.2))
    (:`then_1`
      (bind (_direction _newtrack_0) (`Timeline|OpenCloseDoor` :!via `PlayFromStart`)
        (:`Update`
          (`SceneComponent.K2_SetRelativeRotation` (`self.Locker_Door`) (`KismetMathLibrary.MakeRotator` 0.0 0.0 (`KismetMathLibrary.Lerp` (`self.ClosedAngle`) (`self.OpenAngle`) _newtrack_0)) false false))))))

(event `self.Box.OnComponentBeginOverlap`
  (params (OverlappedComponent :type "PrimitiveComponent Object Reference") (OtherActor :type "Actor Object Reference") (OtherComp :type "PrimitiveComponent Object Reference") (OtherBodyIndex :type Integer) (bFromSweep :type Boolean) (SweepResult :type "HitResult Structure (by ref)"))
  ;[1 1 1] In/OutLocker
)

(event `self.Box.OnComponentEndOverlap`
  (params (OverlappedComponent :type "PrimitiveComponent Object Reference") (OtherActor :type "Actor Object Reference") (OtherComp :type "PrimitiveComponent Object Reference") (OtherBodyIndex :type Integer))
  ;[1 1 1] In/OutLocker
)

(fn `ToggleHide`
  (bind _returnvalue (`GameplayStatics.GetPlayerController` 0))
  (bind _playerref (`self.PlayerRef`))
  (if (`self.IsHiding?`)
    (set `self.IsHiding?` false)
    (`self.SetActorHiddenInGame` _playerref false)
    (`self.SetActorEnableCollision` _playerref true)
    (`PlayerController.SetViewTargetWithBlend` _returnvalue _playerref 0.8 "VTBlend_Linear" 0.0 false)
    (set `/Game/FirstPerson/Blueprints/BP_FirstPersonCharacter.IsHiding` false _playerref)
    (else
      (set `self.IsHiding?` true)
      (`self.SetActorHiddenInGame` _playerref true)
      (`self.SetActorEnableCollision` _playerref false)
      (`PlayerController.SetViewTargetWithBlend` _returnvalue self 0.8 "VTBlend_Linear" 0.0 false)
      (set `/Game/FirstPerson/Blueprints/BP_FirstPersonCharacter.IsHiding` true _playerref))))

(fn `UserConstructionScript`)