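; WinZone is a trigger actor that ends the game with a win screen when the first-person character enters its collision box.
; On overlap it casts to BP_FirstPersonCharacter, stores the reference and stops that character's camera shake.
; A DoOnce then shows the YouWin widget, enables the mouse cursor with Game and UI input focused on it, pauses the game and plays the Sweet_Lamb sound.
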(event `self.CollisionBox.OnComponentBeginOverlap`
  (params (OverlappedComponent :type "PrimitiveComponent Object Reference") (OtherActor :type "Actor Object Reference") (OtherComp :type "PrimitiveComponent Object Reference") (OtherBodyIndex :type Integer) (bFromSweep :type Boolean) (SweepResult :type "HitResult Structure (by ref)"))
  (bind _returnvalue (`GameplayStatics.GetPlayerController` 0))
  (bind _asbp_first_person_character (cast `/Game/FirstPerson/Blueprints/BP_FirstPersonCharacter` OtherActor))
  (bind _output_get (set `self.As BP First Person Character` _asbp_first_person_character))
  (`/Game/FirstPerson/Blueprints/BP_FirstPersonCharacter.StopCamShake` _output_get)
  (`/Engine/EditorBlueprintResources/StandardMacros.DoOnce` false
    (:`Completed`
      (bind _returnvalue_2 (`|CreateWidget` "/Game/Widgets/YouWin.YouWin_C"))
      (`UserWidget.AddToViewport` _returnvalue_2 0)
      (set `PlayerController.bShowMouseCursor` true _returnvalue)
      (`WidgetBlueprintLibrary.SetInputMode_GameAndUIEx` _returnvalue _returnvalue_2)
      (`GameplayStatics.SetGamePaused` true)
      (`GameplayStatics.PlaySound2D` "/Game/AIDoctor/SFX/Sweet_Lamb.Sweet_Lamb" 1.0 1.0 0.0 null null))))

(fn `UserConstructionScript`)