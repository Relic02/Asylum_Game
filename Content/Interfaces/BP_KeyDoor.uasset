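; Key-locked door actor that swings open or closed through its Use event when the using actor has the cage key.
; Use checks HasCageKey and prints a key-needed message if it is false.
; Otherwise the IsDoorClosed flag selects one of two timelines, one played forward and one in reverse, to lerp the Door's yaw between angle variables.
; Each timeline flips the flag when it finishes.
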(event `/Game/Interfaces/InteractInterface.Use`
  (params (Actor :type "/Game/FirstPerson/Blueprints/BP_FirstPersonCharacter Object Reference"))
  (bind _door (`self.Door`))
  (if (`/Game/FirstPerson/Blueprints/BP_FirstPersonCharacter.HasCageKey?` Actor)
    (if (`self.IsDoorClosed`)
      (bind (_direction _open_close) (`Timeline|Timeline_1` :!via `PlayFromStart`)
        (:`Update`
          (`SceneComponent.K2_SetRelativeRotation` _door (`KismetMathLibrary.MakeRotator` 0.0 0.0 (`KismetMathLibrary.Lerp` (`self.OpenAngle`) (`self.ClosedAngle`) _open_close)) false false))
        (:`Finished`
          (set `self.IsDoorClosed` false)))
      (else
        (bind (_direction_2 _open_close_2) (`Timeline|Timeline_2` :!via `ReverseFromEnd`)
          (:`Update`
            (`SceneComponent.K2_SetRelativeRotation` _door (`KismetMathLibrary.MakeRotator` 0.0 0.0 (`KismetMathLibrary.Lerp` (`self.ClosedAngle`) (`self.OpenAngle`) _open_close_2)) false false))
          (:`Finished`
            (set `self.IsDoorClosed` true)))))
    (else
      (`KismetSystemLibrary.PrintString` "Needs a Key"))))

(fn `UserConstructionScript`
  (`parent.UserConstructionScript`))