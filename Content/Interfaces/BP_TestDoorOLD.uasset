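; Test door Blueprint, marked OLD in its name, that swings open or closed when used.
; Its Use function calls OpenDoor, which waits briefly, then branches on IsDoorClosed.
; Separate timelines drive opening and closing, one played forward and the other in reverse, lerping the Door's relative yaw between ClosedAngle and OpenAngle.
; IsDoorClosed flips only when a timeline finishes.
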(event `OpenDoor`
  (`KismetSystemLibrary.Delay` 0.2)
  (if (`self.IsDoorClosed`)
    (bind (_direction _open_close) (`Timeline|DoorOpen` :!via `PlayFromStart`)
      (:`Update`
        (`SceneComponent.K2_SetRelativeRotation` (`self.Door`) (`KismetMathLibrary.MakeRotator` 0.0 0.0 (`KismetMathLibrary.Lerp` (`self.ClosedAngle`) (`self.OpenAngle`) _open_close)) false false))
      (:`Finished`
        (set `self.IsDoorClosed` false)))
    (else
      (bind (_direction_2 _open_close_2) (`Timeline|Timeline_0` :!via `ReverseFromEnd`)
        (:`Update`
          (`SceneComponent.K2_SetRelativeRotation` (`self.Door`) (`KismetMathLibrary.MakeRotator` 0.0 0.0 (`KismetMathLibrary.Lerp` (`self.ClosedAngle`) (`self.OpenAngle`) _open_close_2)) false false))
        (:`Finished`
          (set `self.IsDoorClosed` true))))))

(fn `Use`
  (params (Actor :type "/Game/FirstPerson/Blueprints/BP_FirstPersonCharacter Object Reference"))
  (`self.OpenDoor`)
  (return))

(fn `UserConstructionScript`)