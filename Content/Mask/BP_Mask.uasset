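; BP_Mask is an actor that feeds the world location and scale of its Sphere component to materials, apparently to act as a mask volume.
; It writes both values as vector parameters into a Material Parameter Collection, so any material reading that collection can follow the sphere.
; The write runs in the Construction Script for editor updates and again every Tick at runtime.
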(event `self.ReceiveTick`
  (params (DeltaSeconds :type "Float (single-precision)"))
  (bind _sphere (`self.Sphere`))
  (`KismetMaterialLibrary.SetVectorParameterValue` "/Game/Mask/MaterialParameterCollection.MaterialParameterCollection" "location" (`KismetMathLibrary.Conv_VectorToLinearColor` (`SceneComponent.K2_GetComponentLocation` _sphere)))
  (`KismetMaterialLibrary.SetVectorParameterValue` "/Game/Mask/MaterialParameterCollection.MaterialParameterCollection" "Scale" (`KismetMathLibrary.Conv_VectorToLinearColor` (`SceneComponent.K2_GetComponentScale` _sphere))))

(fn `UserConstructionScript`
  (bind _sphere (`self.Sphere`))
  (`KismetMaterialLibrary.SetVectorParameterValue` "/Game/Mask/MaterialParameterCollection.MaterialParameterCollection" "location" (`KismetMathLibrary.Conv_VectorToLinearColor` (`SceneComponent.K2_GetComponentLocation` _sphere)))
  (`KismetMaterialLibrary.SetVectorParameterValue` "/Game/Mask/MaterialParameterCollection.MaterialParameterCollection" "Scale" (`KismetMathLibrary.Conv_VectorToLinearColor` (`SceneComponent.K2_GetComponentScale` _sphere))))